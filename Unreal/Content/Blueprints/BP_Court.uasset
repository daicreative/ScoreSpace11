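; BP_Court is a tennis court actor that hosts one match and registers itself with BP_GameMode.
; It spawns and attaches its ball, opponent and ballboy, seats the player on court index 0, and moves BallFollow after the ball each tick.
; Points roll into games with win-by-two scoring, updating CourtUI and swapping server each game.
; Match completion is unfinished: GiveMatch is empty and the money payout logic never runs.
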(event EventBeginPlay
  (bind _asbp_game_mode (Utilities|Casting|CastToBP_GameMode (Game|GetGameMode)))
  (Default|SetupCourt _asbp_game_mode self)
  (CallFunction|SpawnBall)
  (CallFunction|SpawnTennisPeople))

(event Collision|EventActorBeginOverlap
  (params (OtherActor :type Actor%20Object%20Reference)))

(event EventTick
  (params (DeltaSeconds :type Float%20%28single-precision%29))
  (CallFunction|BallFollowTick))

(fn ConstructionScript
  (Rendering|Material|SetVectorParameterValueonMaterials (Variables|Default|GetCourt) "Color" (Math|Conversions|ToVector(LinearColor) (Variables|Construction|GetOpponentColor)))
  (Variables|/Script/Engine.SceneCaptureComponent2D|SetTextureTarget (Variables|Default|GetRenderCam) (Variables|Construction|GetRenderTarget)))

(fn SpawnTennisPeople
  (bind _returnvalue (Game|Player|GetPlayerPawn 0))
  (bind _returnvalue_2 (Game|SpawnActorfromClass "/Game/Blueprints/BP_TennisOpponent.BP_TennisOpponent_C" (Transformation|GetRelativeTransform (Variables|Default|GetOpponentSpawn)) "Undefined" 0 0))
  (Transformation|AttachActorToActor _returnvalue_2 self "None" "KeepRelative" "KeepRelative" "KeepRelative" true)
  (bind _returnvalue_3 (Game|SpawnActorfromClass "/Game/Blueprints/BP_Ballboy.BP_Ballboy_C" (Transformation|GetRelativeTransform (Variables|Default|GetBallboySpawn)) "Undefined" 0 0))
  (Transformation|AttachActorToActor _returnvalue_3 self "None" "KeepRelative" "KeepRelative" "KeepRelative" true)
  (if (== (Variables|Construction|GetCourtIndex) 0)
    (Transformation|AttachActorToActor _returnvalue self "None" "KeepRelative" "KeepRelative" "KeepRelative" true)
    (Transformation|SetActorTransform _returnvalue (Transformation|GetWorldTransform (Variables|Default|GetPlayerSpawn)))))

(fn SpawnBall
  (bind _self self)
  (bind _returnvalue (Game|SpawnActorfromClass "/Game/Blueprints/BP_Ball.BP_Ball_C" (Math|Transform|MakeTransform (Transformation|GetWorldLocation (Variables|Default|GetBallSpawn)) "0, 0, 0" (* (Class|KismetMathLibrary|VectorOne) (Variables|Construction|GetBallScale))) "Undefined" 0 0))
  (Transformation|AttachActorToActor _returnvalue _self "None" "KeepWorld" "KeepWorld" "KeepWorld" true)
  (Default|SetupBall _returnvalue _self)
  (Variables|Game|SetCourt%20Ball _returnvalue))

(fn BallFollowTick
  (bind _court_ball (Variables|Game|GetCourt%20Ball))
  (bind _staticmesh (Variables|/Game/Blueprints/BP_Ball.BP_Ball_C|GetStaticMesh _court_ball))
  (bind _returnvalue (Transformation|GetRelativeTransform _staticmesh))
  (Transformation|SetRelativeLocation (Variables|Default|GetBallFollow) (Math|Vector|MakeVector (Math|Float|Max(Float) (.x (.location _returnvalue)) 7.5e+02) (.y (.location _returnvalue)) 0.0) false false))

(fn GivePoint
  (params (Player :type Boolean))
  (bind _court_ball (Variables|Game|GetCourt%20Ball))
  (bind _playerscore (Variables|Game|GetPlayerScore))
  (Variables|/Game/Blueprints/BP_Ball.BP_Ball_C|SetBall%20State _court_ball "NewEnumerator0")
  (Variables|/Game/Blueprints/BP_Ball.BP_Ball_C|SetBounced _court_ball false)
  (if Player
    (bind _result (Math|Integer|IncrementInt _playerscore)
      (:%20%20
        (if (and (> (- _playerscore (Variables|Game|GetOpponentScore)) 1) (> _result 3))
          (CallFunction|GiveGame true))))
    (else
      (bind _result_2 (Math|Integer|IncrementInt (Variables|Game|GetOpponentScore))
        (:%20%20
          (if (and (> (- (Variables|Game|GetOpponentScore) (Variables|Game|GetPlayerScore)) 1) (> _result_2 3))
            (CallFunction|GiveGame false))))))
  (Default|UpdatePointsUI (Variables|Default|GetCourtUI) (Variables|Game|GetPlayerScore) (Variables|Game|GetOpponentScore))
  (Variables|Game|SetPlayerHitsNext (Variables|Game|GetPlayerIsServer)))

(fn GiveGame
  (params (Player :type Boolean))
  (bind _gameindex (Variables|Game|GetGameIndex))
  (bind _games (Variables|Game|GetGames))
  (if Player
    (LocalVariables|SetGame 1)
    (else
      (LocalVariables|SetGame -1)))
  (Utilities|Array|SetArrayElem _games _gameindex (LocalVariables|GetGame))
  (Default|UpdateMatchUI (Variables|Default|GetCourtUI) _gameindex (LocalVariables|GetGame))
  (Math|Integer|IncrementInt _gameindex
    (:%20%20
      (Variables|Game|SetPlayerScore 0)
      (Variables|Game|SetOpponentScore 0)
      (Variables|Game|SetPlayerIsServer (not (Variables|Game|GetPlayerIsServer)))
      (for _array_element _games
        (if (== _array_element -1)
          (Math|Integer|IncrementInt (LocalVariables|GetOpponentWins))
          (elif (== _array_element 1)
            (Math|Integer|IncrementInt (LocalVariables|GetPlayerWins)))))
      (if (not (== (LocalVariables|GetPlayerWins) 2))
        (if (== (LocalVariables|GetOpponentWins) 2)
          _)))))

(fn GiveMatch
  (params (Player :type Boolean)))