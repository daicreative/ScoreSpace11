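; Tennis player character, attached to a BP_Court actor, with a configurable color and walk speed.
; The construction script passes the color to body and racket materials and sets max walk speed.
; Each tick smoothly rotates the mesh: toward zero world rotation when the capsule's relative X is positive, otherwise upright facing the parent court's origin.
; Swing and Serve are empty stubs.
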(event EventBeginPlay)

(event Collision|EventActorBeginOverlap
  (params (OtherActor :type Actor%20Object%20Reference)))

(event EventTick
  (params (DeltaSeconds :type Float%20%28single-precision%29))
  (CallFunction|RotationTick DeltaSeconds))

(fn ConstructionScript
  (bind _color (Variables|Construction|GetColor))
  (bind _returnvalue (Math|Conversions|ToVector(LinearColor) _color))
  (Rendering|Material|SetVectorParameterValueonMaterials (Variables|Default|Gettestbody) "None" _returnvalue)
  (Rendering|Material|SetVectorParameterValueonMaterials (Variables|Default|Getracket) "None" _returnvalue)
  (Variables|/Script/Engine.CharacterMovementComponent|SetMaxWalkSpeed (Variables|Character|GetCharacterMovement) (Variables|Default|GetWalkSpeed)))

(fn Swing)

(fn Serve)

(fn GetCourt
  (bind _asbp_court (Utilities|Casting|CastToBP_Court (Actor|GetAttachParentActor)))
  (return _asbp_court))

(fn RotationTick
  (params (DeltaTime :type Float%20%28single-precision%29))
  (bind _mesh (Variables|Character|GetMesh))
  (bind _returnvalue (Transformation|GetWorldRotation _mesh))
  (if (> (.x (.location (Transformation|GetRelativeTransform (Variables|Collision|GetCapsuleComponent)))) 0.0)
    (Transformation|SetWorldRotation (Variables|Character|GetMesh) (Math|Interpolation|RInterpTo _returnvalue "0, 0, 0" DeltaTime 1e+01) false false)
    (else
      (Transformation|SetWorldRotation (Variables|Character|GetMesh) (Math|Interpolation|RInterpTo _returnvalue (Math|Rotator|MakeRotfromZX (Math|Vector|VectorUp) (- (Math|Transform|TransformLocation (Transformation|GetActorTransform (CallFunction|GetCourt)) "0, 0, 0") (Transformation|GetWorldLocation _mesh))) DeltaTime 6.0) false false))))