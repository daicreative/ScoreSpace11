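; BP_Ball is the ball for a two-sided court game with tennis-like rules, tracking bounces and awarding points through its Court.
; SetupBall derives both half-court rectangles from the Court's corner markers for 2D bounds checks.
; Hits on Court-tagged components run HitGround, which scores out-of-bounds or second bounces during rallies and marks tossed balls dead.
; GetHit clears the bounce and flips whose turn it is when the expected side hits.
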(event OnComponentHit(StaticMesh)
  (params (HitComponent :type Primitive%20Component%20Object%20Reference) (OtherActor :type Actor%20Object%20Reference) (OtherComp :type Primitive%20Component%20Object%20Reference) (NormalImpulse :type Vector :default "0, 0, 0") (Hit :type Hit%20Result%20Structure%20%28by%20ref%29))
  (if (Components|ComponentHasTag OtherComp "Court")
    (CallFunction|HitGround)))

(event EventBeginPlay)

(event Collision|EventActorBeginOverlap
  (params (OtherActor :type Actor%20Object%20Reference)))

(event EventTick
  (params (DeltaSeconds :type Float%20%28single-precision%29)))

(fn ConstructionScript)

(fn OutPlayerArea
  (params (Hit :type Vector%202D%20Structure))
  (bind _bottomleft (Variables|Information|GetBottomLeft))
  (bind _midright (Variables|Information|GetMidRight))
  (return (not (Math|Boolean|ANDBoolean (> (.x Hit) (.x _bottomleft)) (> (.y Hit) (.y _bottomleft)) (< (.x Hit) (.x _midright)) (< (.y Hit) (.y _midright))))))

(fn OutOpponentArea
  (params (Hit :type Vector%202D%20Structure))
  (bind _topright (Variables|Information|GetTopRight))
  (bind _midleft (Variables|Information|GetMidLeft))
  (return (not (Math|Boolean|ANDBoolean (> (.x Hit) (.x _midleft)) (> (.y Hit) (.y _midleft)) (< (.x Hit) (.x _topright)) (< (.y Hit) (.y _topright))))))

(fn SetupBall
  (params (Court :type BP%20Court%20Object%20Reference))
  (bind _output_get (Variables|Default|SetCourt Court))
  (bind _output_get_2 (Variables|Information|SetBottomLeft (Math|Conversions|ToVector2D(Vector) (Transformation|GetWorldLocation (Variables|/Game/Blueprints/BP_Court.BP_Court_C|GetBottomLeft _output_get)))))
  (bind _output_get_3 (Variables|Information|SetTopRight (Math|Conversions|ToVector2D(Vector) (Transformation|GetWorldLocation (Variables|/Game/Blueprints/BP_Court.BP_Court_C|GetTopRight _output_get)))))
  (Variables|Information|SetMidLeft (Math|Vector2D|MakeVector2D (/ (+ (.x _output_get_2) (.x _output_get_3)) 2.0) (.y _output_get_2)))
  (Variables|Information|SetMidRight (Math|Vector2D|MakeVector2D (/ (+ (.x _output_get_2) (.x _output_get_3)) 2.0) (.y _output_get_3))))

(fn GetBallLocation
  (return (Transformation|GetWorldLocation (Variables|Default|GetStaticMesh))))

(fn SetPhysicsState
  (params (State :type Boolean))
  (bind _staticmesh (Variables|Default|GetStaticMesh))
  (Physics|SetSimulatePhysics _staticmesh State)
  (if State
    (Collision|SetCollisionEnabled _staticmesh "QueryAndPhysics")
    (else
      (Collision|SetCollisionEnabled _staticmesh "NoCollision"))))

(fn HitGround
  (bind _court (Variables|Default|GetCourt))
  (bind _playerhitsnext (Variables|/Game/Blueprints/BP_Court.BP_Court_C|GetPlayerHitsNext _court))
  (bind _returnvalue (not _playerhitsnext))
  (switch Utilities|FlowControl|Switch|SwitchonBallState (Variables|Game|GetBall%20State)
    (:NewEnumerator1
      (if (CallFunction|OutOfBounds)
        (if (Variables|Game|GetBounced)
          (Default|GivePoint _court _returnvalue)
          (else
            (Default|GivePoint _court _playerhitsnext)))
        (elif (Variables|Game|GetBounced)
          (Default|GivePoint _court _returnvalue)
          (else
            (Variables|Game|SetBounced true)))))
    (:NewEnumerator3
      (Variables|Game|SetBall%20State "NewEnumerator0"))))

(fn ServingState
  (bind _ball_state (Variables|Game|GetBall%20State))
  (return (Math|Boolean|ORBoolean (Utilities|Enum|Equal(Enum) _ball_state "NewEnumerator0") (Utilities|Enum|Equal(Enum) _ball_state "NewEnumerator2") (Utilities|Enum|Equal(Enum) _ball_state "NewEnumerator3"))))

(fn OutOfBounds
  (bind _staticmesh (Variables|Default|GetStaticMesh))
  (bind _returnvalue (Transformation|GetWorldLocation _staticmesh))
  (bind _returnvalue_2 (Math|Conversions|ToVector2D(Vector) _returnvalue))
  (if (Variables|/Game/Blueprints/BP_Court.BP_Court_C|GetPlayerHitsNext (Variables|Default|GetCourt))
    (return (CallFunction|OutPlayerArea _returnvalue_2))
    (else
      (return (CallFunction|OutOpponentArea _returnvalue_2)))))

(fn GetHit
  (params (PlayerHit :type Boolean))
  (bind _court (Variables|Default|GetCourt))
  (if (Utilities|Enum|Equal(Enum) (Variables|Game|GetBall%20State) "NewEnumerator1")
    (if (Math|Boolean|Equal(Boolean) (Variables|/Game/Blueprints/BP_Court.BP_Court_C|GetPlayerHitsNext _court) PlayerHit)
      (Variables|Game|SetBounced false)
      (Variables|/Game/Blueprints/BP_Court.BP_Court_C|SetPlayerHitsNext _court (not (Variables|/Game/Blueprints/BP_Court.BP_Court_C|GetPlayerHitsNext _court))))))