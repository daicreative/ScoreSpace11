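; AI controller for a tennis opponent pawn that runs the tennis behavior tree on possession and handles an "assaulted" interruption.
; AssaultedAI stops the behavior tree logic and starts a 20-second countdown.
; Tick counts the timer down and feeds it to the opponent's assault count; at zero it clears the pawn's assaulted state and restarts the brain logic.
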(event EventBeginPlay)

(event EventTick
  (params (DeltaSeconds :type Float%20%28single-precision%29))
  (bind _possessed (Variables|Default|GetPossessed))
  (bind _output_get (Variables|Default|SetTimer (Math|Float|Max(Float) (- (Variables|Default|GetTimer) DeltaSeconds) 0.0)))
  (Default|UpdateAssaultCount _possessed _output_get)
  (if (and (Variables|Default|GetTimerSet) (== _output_get 0.0))
    (Variables|Default|SetTimerSet false)
    (Default|Assaulted _possessed false "0, 0, 0" false)
    (Class|BrainComponent|RestartLogic (Variables|Default|GetBrainComponent))))

(event EventPossess
  (params (PossessedPawn :type Pawn%20Object%20Reference))
  (bind _asbp_tennis_opponent (Utilities|Casting|CastToBP_TennisOpponent PossessedPawn))
  (Variables|Default|SetPossessed _asbp_tennis_opponent)
  (AI|RunBehaviorTree "/Game/Blueprints/AI/TennisAIBehaviorTree.TennisAIBehaviorTree"))

(fn ConstructionScript)

(fn AssaultedAI
  (Variables|Default|SetTimerSet true)
  (Variables|Default|SetTimer 2e+01)
  (AI|Logic|StopLogic (Variables|Default|GetBrainComponent) ""))