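; AI controller for the ballboy character that runs its behavior tree on possession and handles it being assaulted.
; AssaultedAI stops the brain logic and starts a countdown timer.
; Tick counts the timer down, then clears the ballboy's assaulted state with zero impulse and restarts the behavior tree.
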(event EventBeginPlay)

(event EventTick
  (params (DeltaSeconds :type Float%20%28single-precision%29))
  (Variables|Default|SetTimer (Math|Float|Max(Float) (- (Variables|Default|GetTimer) DeltaSeconds) 0.0))
  (if (and (Variables|Default|GetTimerSet) (== (Variables|Default|GetTimer) 0.0))
    (Variables|Default|SetTimerSet false)
    (Default|Assaulted (Variables|Default|GetPossessed) false "0, 0, 0")
    (Class|BrainComponent|RestartLogic (Variables|Default|GetBrainComponent))))

(event EventPossess
  (params (PossessedPawn :type Pawn%20Object%20Reference))
  (bind _asbp_ballboy (Utilities|Casting|CastToBP_Ballboy PossessedPawn))
  (Variables|Default|SetPossessed _asbp_ballboy)
  (AI|RunBehaviorTree "/Game/Blueprints/AI/BallboyBehaviorTree.BallboyBehaviorTree"))

(fn ConstructionScript)

(fn AssaultedAI
  (Variables|Default|SetTimerSet true)
  (Variables|Default|SetTimer 15.0)
  (AI|Logic|StopLogic (Variables|Default|GetBrainComponent) ""))