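; BP_CourtPerson is a character on a BP_Court that can pick up and drop that court's ball.
; PickupTrigger's begin and end overlaps both set BallInRange from the other actor's Ball tag, so leaving does not clear it.
; PickupBall and DropBall change the ball's state and HasBall, attaching it to the hand-off socket or back to the parent court.
; Construction applies walk speed and pushes Color to an unnamed material parameter.
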(event OnComponentBeginOverlap(PickupTrigger)
  (params (OverlappedComponent :type Primitive%20Component%20Object%20Reference) (OtherActor :type Actor%20Object%20Reference) (OtherComp :type Primitive%20Component%20Object%20Reference) (OtherBodyIndex :type Integer) (bFromSweep :type Boolean) (SweepResult :type Hit%20Result%20Structure%20%28by%20ref%29))
  (Variables|Tennis|SetBallInRange (Actor|ActorHasTag OtherActor "Ball")))

(event OnComponentEndOverlap(PickupTrigger)
  (params (OverlappedComponent :type Primitive%20Component%20Object%20Reference) (OtherActor :type Actor%20Object%20Reference) (OtherComp :type Primitive%20Component%20Object%20Reference) (OtherBodyIndex :type Integer))
  (Variables|Tennis|SetBallInRange (Actor|ActorHasTag OtherActor "Ball")))

(event EventBeginPlay)

(event Collision|EventActorBeginOverlap
  (params (OtherActor :type Actor%20Object%20Reference)))

(event EventTick
  (params (DeltaSeconds :type Float%20%28single-precision%29)))

(fn ConstructionScript
  (bind _color (Variables|Construction|GetColor))
  (bind _mesh (Variables|Character|GetMesh))
  (bind _returnvalue (Math|Conversions|ToVector(LinearColor) _color))
  (Rendering|Material|SetVectorParameterValueonMaterials _mesh "None" _returnvalue)
  (Rendering|Material|SetVectorParameterValueonMaterials _mesh "None" _returnvalue)
  (Variables|/Script/Engine.CharacterMovementComponent|SetMaxWalkSpeed (Variables|Character|GetCharacterMovement) (Variables|Default|GetWalkSpeed)))

(fn GetCourt
  (bind _asbp_court (Utilities|Casting|CastToBP_Court (Actor|GetAttachParentActor)))
  (return _asbp_court))

(fn PickupBall
  (bind _court (CallFunction|GetCourt))
  (bind _court_ball (Variables|/Game/Blueprints/BP_Court.BP_Court_C|GetCourt%20Ball _court))
  (Variables|/Game/Blueprints/BP_Ball.BP_Ball_C|SetBall%20State _court_ball "NewEnumerator2")
  (Transformation|AttachActorToActor _court_ball self "ball_Socket" "KeepRelative" "KeepRelative" "KeepRelative" true)
  (Variables|Tennis|SetHasBall true))

(fn DropBall
  (bind _court (CallFunction|GetCourt))
  (bind _court_ball (Variables|/Game/Blueprints/BP_Court.BP_Court_C|GetCourt%20Ball _court))
  (Variables|/Game/Blueprints/BP_Ball.BP_Ball_C|SetBall%20State _court_ball "NewEnumerator0")
  (Transformation|DetachFromActor _court_ball "KeepWorld" "KeepWorld" "KeepWorld")
  (Transformation|AttachActorToActor _court_ball _court "None" "KeepWorld" "KeepWorld" "KeepWorld" true)
  (Variables|Tennis|SetHasBall false))