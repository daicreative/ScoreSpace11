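; Game mode that owns the main GameUI widget and routes per-court render materials into it.
; The construction script creates GameUI and adds it to the viewport, while BeginPlay sets game-only input and hides the mouse cursor.
; SetupCourtUI-GameMode looks up a court widget by index in GameUI and passes it the render material and that index.
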(event EventBeginPlay
  (bind _returnvalue (Game|GetPlayerController 0))
  (Input|SetInputModeGameOnly _returnvalue)
  (Variables|/Script/Engine.PlayerController|SetbShowMouseCursor _returnvalue false))

(event EventTick
  (params (DeltaSeconds :type Float%20%28single-precision%29)))

(fn ConstructionScript
  (CallFunction|SetupUI))

(fn SetupUI
  (bind _returnvalue (UserInterface|CreateWidget "/Game/UI/GameUI.GameUI_C"))
  (bind _output_get (Variables|UI|SetGameUI _returnvalue))
  (UserInterface|Viewport|AddtoViewport _output_get 0))

(fn SetupCourtUI-GameMode
  (params (RenderMaterial :type Material%20Object%20Reference) (Integer :type Integer))
  (bind _ui (Default|GetCourtUIbyIndex (Variables|UI|GetGameUI) Integer))
  (Default|SetupCourtUI _ui RenderMaterial Integer))