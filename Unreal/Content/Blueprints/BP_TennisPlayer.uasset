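; BP_TennisPlayer is the input-driven tennis player character, able to swing at balls and assault ballboys or opponents.
; Input drives movement, swing and ball actions, a ragdoll toggle, and a sprint with a draining, recharging meter updated on Tick.
; A Box overlap flags tagged balls as hittable and stores nearby ballboys or opponents.
; Swinging also notifies a stored victim's AI controller and launches them forward and up through Assaulted.
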(event OnComponentBeginOverlap(Box)
  (params (OverlappedComponent :type Primitive%20Component%20Object%20Reference) (OtherActor :type Actor%20Object%20Reference) (OtherComp :type Primitive%20Component%20Object%20Reference) (OtherBodyIndex :type Integer) (bFromSweep :type Boolean) (SweepResult :type Hit%20Result%20Structure%20%28by%20ref%29))
  (if (Components|ComponentHasTag OtherComp "Ball")
    (Variables|Default|SetBallHittable true)
    (else
      (bind _asbp_ballboy (Utilities|Casting|CastToBP_Ballboy OtherActor)
        (:then
          (Variables|Default|SetAssaultBallboy _asbp_ballboy))
        (:CastFailed
          (bind _asbp_tennis_opponent (Utilities|Casting|CastToBP_TennisOpponent OtherActor))
          (Variables|Default|SetAssaultOpponent _asbp_tennis_opponent))))))

(event OnComponentEndOverlap(Box)
  (params (OverlappedComponent :type Primitive%20Component%20Object%20Reference) (OtherActor :type Actor%20Object%20Reference) (OtherComp :type Primitive%20Component%20Object%20Reference) (OtherBodyIndex :type Integer))
  (if (Components|ComponentHasTag OtherComp "Ball")
    (Variables|Default|SetBallHittable false)
    (else
      (Utilities|Casting|CastToBP_Ballboy OtherActor
        (:then
          (Variables|Default|SetAssaultBallboy 0))
        (:CastFailed
          (Utilities|Casting|CastToBP_TennisOpponent OtherActor)
          (Variables|Default|SetAssaultOpponent 0))))))

(event EventBeginPlay)

(event Collision|EventActorBeginOverlap
  (params (OtherActor :type Actor%20Object%20Reference)))

(event EventTick
  (params (DeltaSeconds :type Float%20%28single-precision%29))
  (|CallParentFunction DeltaSeconds)
  (CallFunction|SprintTick DeltaSeconds))

(event Input|ActionEvents|InputActionBallAction
  (params (Key :type Key%20Structure :default "None"))
  (:Pressed
    (CallFunction|BallAction)))

(event Input|ActionEvents|InputActionSwing
  (params (Key :type Key%20Structure :default "None"))
  (:Pressed
    (CallFunction|SwingAction)
    (Utilities|IsValid (Variables|Default|GetAssaultBallboy)
      (:Is%20Valid
        (CallFunction|HitBallboy))
      (:Is%20Not%20Valid
        _))
    (Utilities|IsValid (Variables|Default|GetAssaultOpponent)
      (:Is%20Valid
        (CallFunction|HitOpponent)))))

(event Input|ActionEvents|InputActionSprint
  (params (Key :type Key%20Structure :default "None"))
  (bind _charactermovement (Variables|Character|GetCharacterMovement))
  (bind _sprintspeed (Variables|Sprint|GetSprintSpeed))
  (:Pressed
    (if (> (Variables|Sprint|GetSprint) 0.0)
      (Variables|Sprint|SetSprinting true)
      (Variables|/Script/Engine.CharacterMovementComponent|SetMaxWalkSpeed _charactermovement _sprintspeed)
      (Variables|/Script/Engine.MovementComponent|SetVelocity _charactermovement (* (Math|Vector|Normalize (Variables|/Script/Engine.MovementComponent|GetVelocity _charactermovement)) _sprintspeed))))
  (:Released
    (Variables|Sprint|SetSprinting false)
    (Variables|/Script/Engine.CharacterMovementComponent|SetMaxWalkSpeed (Variables|Character|GetCharacterMovement) (Variables|Default|GetWalkSpeed))))

(event Input|ActionEvents|InputActionRagdoll
  (params (Key :type Key%20Structure :default "None"))
  (:Pressed
    (CallFunction|Assaulted true "0, 0, 0"))
  (:Released
    (CallFunction|Assaulted false "0, 0, 0")))

(event Input|AxisEvents|InputAxisHorizontal
  (params (AxisValue :type Float%20%28single-precision%29))
  (Pawn|Input|AddMovementInput (Transformation|GetActorRightVector) AxisValue false))

(event Input|AxisEvents|InputAxisVertical
  (params (AxisValue :type Float%20%28single-precision%29))
  (Pawn|Input|AddMovementInput (Transformation|GetActorForwardVector) AxisValue false))

(fn ConstructionScript
  (|CallParentFunction))

(fn SprintTick
  (params (Delta%20Seconds :type Float%20%28single-precision%29))
  (if (Variables|Sprint|GetSprinting)
    (bind _output_get (Variables|Sprint|SetSprint (Math|Float|Clamp(Float) (- (Variables|Sprint|GetSprint) (* (Variables|Sprint|GetSprintRate) Delta%20Seconds)))))
    (if (== _output_get 0.0)
      (Variables|Sprint|SetSprinting false)
      (Variables|/Script/Engine.CharacterMovementComponent|SetMaxWalkSpeed (Variables|Character|GetCharacterMovement) (Variables|Default|GetWalkSpeed)))
    (else
      (Variables|Sprint|SetSprint (Math|Float|Clamp(Float) (+ (Variables|Sprint|GetSprint) (* (Variables|Sprint|GetSprintRecovery) Delta%20Seconds)))))))

(fn HitBallboy
  (bind _assaultballboy (Variables|Default|GetAssaultBallboy))
  (bind _asballboy_aicontroller (Utilities|Casting|CastToBallboyAIController (AI|GetAIController _assaultballboy)))
  (Default|AssaultedAI _asballboy_aicontroller)
  (Default|Assaulted _assaultballboy true (* (+ (Transformation|GetActorForwardVector) (Math|Vector|VectorUp)) 1e+03)))

(fn HitOpponent
  (bind _assaultopponent (Variables|Default|GetAssaultOpponent))
  (bind _astennis_aicontroller (Utilities|Casting|CastToTennisAIController (AI|GetAIController _assaultopponent)))
  (Default|AssaultedAI _astennis_aicontroller)
  (Default|Assaulted _assaultopponent true (* (+ (Transformation|GetActorForwardVector) (Math|Vector|VectorUp)) 1e+03)))